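; BP_Spawner scatters random meshes from a list onto the ground within a range around itself.
; SpawnObjects randomizes XY and scale, rejects spots where a sphere trace at Z=0 hits "ObjectSpawn"-tagged components, then line-traces down for ground.
; Each placement spawns another BP_Spawner with a random mesh and zero rotation, discarding the generated random rotation.
; A failure limit prevents endless retries; BeginPlay, Tick and the construction script are empty.
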(event `self.ReceiveBeginPlay`)

(event `self.ReceiveTick`
  (params (DeltaSeconds :type "Float (single-precision)")))

(fn `Generate New Transform`
  (returns (`Output Transform` :type "Transform Structure"))
  (bind (_returnvalue_x _returnvalue_y) (`KismetMathLibrary.BreakVector` (`self.K2_GetActorLocation`)))
  (bind (_returnvalue_roll _returnvalue_pitch _returnvalue_yaw) (`KismetMathLibrary.BreakRotator` (`self.K2_GetActorRotation`)))
  (bind _rotation_range (`self.Rotation Range`))
  (bind _scale_range (`self.Scale Range`))
  (bind _returnvalue (* (`self.Spawn Range`) -1.0))
  (bind _returnvalue_2 (`KismetMathLibrary.RandomFloatInRange` (* _rotation_range -1.0) _rotation_range))
  (return (`KismetMathLibrary.MakeTransform` (`KismetMathLibrary.MakeVector` (+ _returnvalue_x (`KismetMathLibrary.RandomFloatInRange` _returnvalue (`self.Spawn Range`))) (+ _returnvalue_y (`KismetMathLibrary.RandomFloatInRange` _returnvalue (`self.Spawn Range`))) 10000.0) (`KismetMathLibrary.MakeRotator` _returnvalue_2 _returnvalue_2 _returnvalue_2) (`KismetMathLibrary.MakeVector` (+ _returnvalue_roll (`KismetMathLibrary.RandomFloatInRange` 0.1 _scale_range)) (+ _returnvalue_pitch (`KismetMathLibrary.RandomFloatInRange` 0.1 _scale_range)) (+ _returnvalue_yaw (`KismetMathLibrary.RandomFloatInRange` 0.1 _scale_range))))))

(fn `IsOverlap?`
  (params (Start :type "Vector Structure"))
  (returns (`IsOverlap?` :type Boolean))
  ; Checking if the next object can be spawned
  (bind _outhits (`KismetSystemLibrary.SphereTraceMultiForObjects` :`Start` Start :`End` Start :`Radius` 70.0 :`ObjectTypes` (`self.AttachToObj`) :`DrawDebugType` "ForDuration"))
  (for _array_element _outhits
    (if (`ActorComponent.ComponentHasTag` (`.HitComponent` (`GameplayStatics.BreakHitResult` _array_element)) "ObjectSpawn")
      (return true)))
  (return false))

(fn `SpawnObjects`
  (locals (Count :type Integer) (`New Obj Transform` :type "Transform Structure") (LoopLimit :type Integer :default 100) (SpawnedObjectCount :type Integer))
  (if (> (`KismetArrayLibrary.Array_Length` (`self.ListOfObjects`)) 0)
    (set `local.Count` (`self.Object Count`))
    (while (and (!= (`local.Count`) 0) (> (`local.LoopLimit`) 0))
      (bind _output_transform (`self.Generate New Transform`))
      (bind _output_get (set `local.New Obj Transform` _output_transform))
      (bind _isoverlap_ (`self.IsOverlap?` (`KismetMathLibrary.MakeVector` (.x (.location _output_get)) (.y (.location _output_get)))))
      (if _isoverlap_
        (`KismetSystemLibrary.PrintString` "Overlap! Object didn't spawned" true true (struct :`R` 1.0 :`G` 0.815304 :`A` 1.0))
        (set `local.LoopLimit` (- (`local.LoopLimit`) 1))
        (else
          (bind _returnvalue (`KismetMathLibrary.MakeVector` (.x (.location _output_get)) (.y (.location _output_get)) (.z (.location _output_get))))
          ; Finding ground to initialize Z
          (bind (_outhit _returnvalue_2) (`KismetSystemLibrary.LineTraceSingleForObjects` :`Start` _returnvalue :`End` (+ _returnvalue (* 150000.0 (* -1 (`self.GetActorUpVector`)))) :`ObjectTypes` (`self.AttachToObj`) :`DrawDebugType` "ForDuration"))
          (if _returnvalue_2
            (bind _returnvalue_3 (`|SpawnActorFromClass` :`Class` "BP_Spawner_C" :`SpawnTransform` (`KismetMathLibrary.MakeTransform` (`.ImpactPoint` (`GameplayStatics.BreakHitResult` _outhit)) (struct) (.scale _output_get)) :`CollisionHandlingOverride` "AlwaysSpawn" :`TransformScaleMethod` "MultiplyWithRoot" :`Instigator` null))
            (`StaticMeshComponent.SetStaticMesh` (`/Game/Tasks/Task_4/BP_Spawner.StaticMesh` _returnvalue_3) (`KismetArrayLibrary.Array_Random` (`self.ListOfObjects`)))
            (set `local.Count` (- (`local.Count`) 1))
            (set `local.SpawnedObjectCount` (+ (`local.SpawnedObjectCount`) 1))
            (else
              (set `local.LoopLimit` (- (`local.LoopLimit`) 1))
              (`KismetSystemLibrary.PrintString` "Object didnt' found the ground" true true (struct :`R` 1.0 :`G` 0.867519 :`B` 0.103622 :`A` 1.0)))))))
    (`KismetSystemLibrary.PrintText` (`|FormatText` "Objects spawned: {0}" (`local.SpawnedObjectCount`)))
    (`KismetSystemLibrary.PrintString` "End Spawn" true true (struct :`G` 1.0 :`B` 0.09978 :`A` 1.0))
    (else
      (`KismetSystemLibrary.PrintString` "The object array is empty!" true true (struct :`R` 1.0 :`B` 0.064041 :`A` 1.0)))))

(fn `UserConstructionScript`)